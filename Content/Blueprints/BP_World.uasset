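; BP_World wires an on-screen settings widget to procedural world generation through its WorldCreator and PerlinNoise references.
; BeginPlay creates BP_Sliders and binds its height slider, random-seed checkbox, and text boxes for seed, X/Y vertex counts and grid spacing.
; Each handler updates WorldCreator or the PerlinNoise seed, then rebuilds through a shared CreateWorld call.
; The checkbox also toggles manual seed entry, restoring a default seed when re-enabled.
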(event Custom|OnTextCommitted_Event_SeedTextBox
  (params (Text :type Text%20%28by%20ref%29) (CommitMethod :type ETextCommit%20Enum :default "Default"))
  ;[1 1 1] Bind to on text committed event of seed text box
  (Class|PerlinNoiseComponent|SetSeed (Variables|Default|GetPerlinNoise) (Math|Conversions|ToInteger(Byte) (Utilities|String|ToString(Text) Text)))
  (Class|WorldCreator|CreateWorld (Variables|Default|GetWorldCreator)))

(event Custom|OnTextCommitted_Event_NumX
  (params (Text :type Text%20%28by%20ref%29) (CommitMethod :type ETextCommit%20Enum :default "Default"))
  (bind _worldcreator (Variables|Default|GetWorldCreator))
  (Variables|/Script/PerlinNoiseWorld.WorldCreator|SetNumberOfVertsInX _worldcreator (Class|KismetMathLibrary|ToInt64(Integer) (Math|Conversions|ToInteger(Byte) (Utilities|String|ToString(Text) Text))))
  (Class|WorldCreator|CreateWorld _worldcreator))

(event Custom|OnTextCommitted_Event_NumY
  (params (Text :type Text%20%28by%20ref%29) (CommitMethod :type ETextCommit%20Enum :default "Default"))
  (bind _worldcreator (Variables|Default|GetWorldCreator))
  (Variables|/Script/PerlinNoiseWorld.WorldCreator|SetNumberOfVertsInY _worldcreator (Class|KismetMathLibrary|ToInt64(Integer) (Math|Conversions|ToInteger(Byte) (Utilities|String|ToString(Text) Text))))
  (Class|WorldCreator|CreateWorld _worldcreator))

(event Custom|OnValueChanged_Height
  (params (Value :type Float%20%28single-precision%29))
  (bind _worldcreator (Variables|Default|GetWorldCreator))
  ;[1 1 1] Bind to on value changed of height slider
  (Variables|/Script/PerlinNoiseWorld.WorldCreator|SetMaxHeight _worldcreator Value)
  (Class|WorldCreator|CreateWorld _worldcreator))

(event Custom|OnCheckStateChanged_RandomSeed
  (params (bIsChecked :type Boolean))
  (bind _perlinnoise (Variables|Default|GetPerlinNoise))
  (bind _uiwidgets (Variables|Default|GetUIWidgets))
  (bind _seedtextbox (Variables|/Game/Blueprints/BP_Sliders.BP_Sliders_C|GetSeedTextBox _uiwidgets))
  ;[1 1 1] Bind to on check changed of random seed check box
  (Utilities|FlowControl|Sequence
    (:then_0
      (bind _output_get (Variables|/Script/PerlinNoiseWorld.PerlinNoiseComponent|SetgenerateRandomSeed _perlinnoise bIsChecked))
      (if _output_get
        (Class|PerlinNoiseComponent|CreateRandomSeed _perlinnoise)
        (else
          (Class|PerlinNoiseComponent|SetSeed _perlinnoise)))
      (Class|WorldCreator|CreateWorld (Variables|Default|GetWorldCreator) :!label _label))
    (:then_1
      (Widget|SetIsEnabled _seedtextbox (not bIsChecked))
      (if (Variables|/Script/UMG.Widget|GetbIsEnabled _seedtextbox)
        (Rendering|Components|TextRender|SetText _seedtextbox "4532")
        (Class|PerlinNoiseComponent|SetSeed _perlinnoise (Math|Conversions|ToInteger(Byte) (Utilities|String|ToString(Text) (Class|EditableTextBox|GetText _seedtextbox))))
        (goto _label)))))

(event Custom|OnTextCommitted_Event_GridSpcaing
  (params (Text :type Text%20%28by%20ref%29) (CommitMethod :type ETextCommit%20Enum :default "Default"))
  (bind _worldcreator (Variables|Default|GetWorldCreator))
  (Variables|/Script/PerlinNoiseWorld.WorldCreator|SetGridSpacing _worldcreator (Math|Conversions|ToFloat(Integer) (Utilities|String|ToString(Text) Text)))
  (Class|WorldCreator|CreateWorld _worldcreator))

(event EventBeginPlay
  (Utilities|FlowControl|Sequence
    (:then_0
      (bind _returnvalue (UserInterface|CreateWidget "/Game/Blueprints/BP_Sliders.BP_Sliders_C"))
      (bind _output_get (Variables|Default|SetUIWidgets _returnvalue))
      (UserInterface|Viewport|AddtoViewport _output_get 0))
    (:then_1
      ;[1 1 1] Bind to on value changed of height slider
      (EventDispatchers|AssignOnValueChanged (Variables|/Game/Blueprints/BP_Sliders.BP_Sliders_C|GetHeightMap_Slider (Variables|Default|GetUIWidgets)) (delegate Custom|OnValueChanged_Height)))
    (:then_2
      ;[1 1 1] Bind to on check changed of random seed check box
      (EventDispatchers|AssignOnCheckStateChanged (Variables|/Game/Blueprints/BP_Sliders.BP_Sliders_C|GetRandomSeedCheck (Variables|Default|GetUIWidgets)) (delegate Custom|OnCheckStateChanged_RandomSeed)))
    (:then_3
      ;[1 1 1] Bind to on text committed event of seed text box
      (EventDispatchers|AssignOnTextCommitted (Variables|/Game/Blueprints/BP_Sliders.BP_Sliders_C|GetSeedTextBox (Variables|Default|GetUIWidgets)) (delegate Custom|OnTextCommitted_Event_SeedTextBox)))
    (:then_4
      (EventDispatchers|AssignOnTextCommitted (Variables|/Game/Blueprints/BP_Sliders.BP_Sliders_C|GetNumXTextBox (Variables|Default|GetUIWidgets)) (delegate Custom|OnTextCommitted_Event_NumX)))
    (:then_5
      (EventDispatchers|AssignOnTextCommitted (Variables|/Game/Blueprints/BP_Sliders.BP_Sliders_C|GetNumYTextBox (Variables|Default|GetUIWidgets)) (delegate Custom|OnTextCommitted_Event_NumY)))
    (:then_6
      (EventDispatchers|AssignOnTextCommitted (Variables|/Game/Blueprints/BP_Sliders.BP_Sliders_C|GetGridSpacingTextBox (Variables|Default|GetUIWidgets)) (delegate Custom|OnTextCommitted_Event_GridSpcaing)))))

(event Collision|EventActorBeginOverlap
  (params (OtherActor :type Actor%20Object%20Reference)))

(event EventTick
  (params (DeltaSeconds :type Float%20%28single-precision%29)))

(fn ConstructionScript)